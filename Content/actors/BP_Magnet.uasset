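; BP_Magnet is a magnet actor that pulls vehicles along the direction of its Arrow component.
; When an actor tagged Vehicle enters Pull_area, it stores the overlapped component and starts a looping timer that applies a mass-independent force to it at short intervals.
; When a vehicle leaves, the timer pauses after a brief delay.
; It tracks one component and timer handle at a time, and prints a debug message on each pull.
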(event `Stop pulling`
  (`KismetSystemLibrary.K2_PauseTimerHandle` (stale `self.pull_area.OnComponentBeginOverlap` _returnvalue)))

(event `self.pull_area.OnComponentBeginOverlap`
  (params (OverlappedComponent :type "PrimitiveComponent Object Reference") (OtherActor :type "Actor Object Reference") (OtherComp :type "PrimitiveComponent Object Reference") (OtherBodyIndex :type Integer) (bFromSweep :type Boolean) (SweepResult :type "HitResult Structure (by ref)"))
  (if (`self.ActorHasTag` OtherActor "Vehicle")
    (bind _output_get (set `self.car mesh` OtherComp))
    (bind _returnvalue (`KismetSystemLibrary.K2_SetTimerDelegate` (delegate `Pull the car Ones`) 0.2 true))))

(event `Pull the car Ones`
  (`PrimitiveComponent.AddForce` (stale `self.pull_area.OnComponentBeginOverlap` _output_get) (* (`SceneComponent.GetForwardVector` (`self.Arrow`)) 30000.0) "None" true)
  (`KismetSystemLibrary.PrintString` "Pulling the car"))

(event `self.pull_area.OnComponentEndOverlap`
  (params (OverlappedComponent :type "PrimitiveComponent Object Reference") (OtherActor :type "Actor Object Reference") (OtherComp :type "PrimitiveComponent Object Reference") (OtherBodyIndex :type Integer))
  (if (`self.ActorHasTag` OtherActor "Vehicle")
    (`KismetSystemLibrary.Delay` 0.2)
    (`self.Stop pulling`)))

(fn `UserConstructionScript`)